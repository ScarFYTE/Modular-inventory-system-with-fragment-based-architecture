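; Consumable item fragment for the inventory system that heals the character who uses it.
; ExecuteAction casts the instigator to BP_ThirdPersonCharacter, adds HealAmount to Health with a hard-coded cap, and prints debug messages.
; It returns one enum result when the heal is applied and another when the cast fails.
; GetActionData supplies the fragment's action text.
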(fn ExecuteAction
  (params (Instigator :type Actor%20Object%20Reference))
  (Development|PrintString 0 "exectued")
  (bind _asbp_third_person_character (Utilities|Casting|CastToBP_ThirdPersonCharacter Instigator)
    (:then
      (if (> (+ (Variables|/Game/ThirdPerson/Blueprints/BP_ThirdPersonCharacter.BP_ThirdPersonCharacter_C|GetHealth _asbp_third_person_character) (Variables|Default|GetHeal%20Amount)) 1e+02)
        (bind _output_get (Variables|/Game/ThirdPerson/Blueprints/BP_ThirdPersonCharacter.BP_ThirdPersonCharacter_C|SetHealth _asbp_third_person_character 1e+02))
        (Development|PrintString 0 (Utilities|String|ToString(Float) _output_get))
        (else
          (bind _output_get_2 (Variables|/Game/ThirdPerson/Blueprints/BP_ThirdPersonCharacter.BP_ThirdPersonCharacter_C|SetHealth _asbp_third_person_character (+ (Variables|/Game/ThirdPerson/Blueprints/BP_ThirdPersonCharacter.BP_ThirdPersonCharacter_C|GetHealth _asbp_third_person_character) (Variables|Default|GetHeal%20Amount))))
          (Development|PrintString 0 (Utilities|String|ToString(Float) _output_get_2))))
      (return "NewEnumerator2"))
    (:CastFailed
      (return "NewEnumerator1"))))

(fn GetActionData
  (return (Variables|Default|GetActionText)))