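; BP_ItemPickup is a world item pickup in the inventory system, showing the mesh of its assigned item definition.
; The mesh comes from the definition's BP_ItemFragment_Mesh fragment, applied in the construction script and again through the RefreshPickupVisuals event.
; Overlapping InteractZone registers the pickup as the third-person character's NearByItem, and leaving it clears that reference.
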(event OnComponentBeginOverlap(InteractZone)
  (params (OverlappedComponent :type Primitive%20Component%20Object%20Reference) (OtherActor :type Actor%20Object%20Reference) (OtherComp :type Primitive%20Component%20Object%20Reference) (OtherBodyIndex :type Integer) (bFromSweep :type Boolean) (SweepResult :type Hit%20Result%20Structure%20%28by%20ref%29))
  (bind _asbp_third_person_character (Utilities|Casting|CastToBP_ThirdPersonCharacter OtherActor))
  (Variables|/Game/ThirdPerson/Blueprints/BP_ThirdPersonCharacter.BP_ThirdPersonCharacter_C|SetNearByItem _asbp_third_person_character self))

(event OnComponentEndOverlap(InteractZone)
  (params (OverlappedComponent :type Primitive%20Component%20Object%20Reference) (OtherActor :type Actor%20Object%20Reference) (OtherComp :type Primitive%20Component%20Object%20Reference) (OtherBodyIndex :type Integer))
  (bind _asbp_third_person_character (Utilities|Casting|CastToBP_ThirdPersonCharacter OtherActor))
  (Variables|/Game/ThirdPerson/Blueprints/BP_ThirdPersonCharacter.BP_ThirdPersonCharacter_C|SetNearByItem _asbp_third_person_character 0))

(event Custom|RefreshPickupVisuals
  (CallFunction|UpdateVisuals))

(fn ConstructionScript
  (CallFunction|UpdateVisuals))

(fn UpdateVisuals
  (bind _itemdef (Variables|Default|GetItemDef))
  (Utilities|IsValid _itemdef
    (:Is%20Valid
      (Components|StaticMesh|SetStaticMesh (Variables|Default|GetStaticMesh) (Variables|/Game/InventorySystem/Fragments/BP_ItemFragment_Mesh.BP_ItemFragment_Mesh_C|GetItem%20Mesh (Class|ItemDefinition|FindFragmentbyClassBP _itemdef "/Game/InventorySystem/Fragments/BP_ItemFragment_Mesh.BP_ItemFragment_Mesh_C"))))))